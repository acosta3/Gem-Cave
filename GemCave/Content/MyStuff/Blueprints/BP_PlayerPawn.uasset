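; BP_PlayerPawn is a player pawn driven by physics forces at two wheels, using forward/backward and turn inputs.
; BeginPlay adds IMC_Default to the first player controller's Enhanced Input subsystem.
; Both Triggered events share one tank-style mix, clamping the sum and difference of action values into left and right wheel forces.
; These are scaled and applied to PlayerMesh at each wheel's location; releasing either input zeroes both values.
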(event Input|EnhancedActionEvents|EnhancedInputActionIA_ForwardsBackwards
  (params (ActionValue :type Float%20%28double-precision%29) (ElapsedSeconds :type Float%20%28double-precision%29) (TriggeredSeconds :type Float%20%28double-precision%29) (InputAction :type Input%20Action%20Object%20Reference :default "/Game/MyStuff/Input/IA_ForwardsBackwards.IA_ForwardsBackwards"))
  (:Triggered
    (bind _output_get (Variables|Default|SetLeftWheelForce (Math|Float|Clamp(Float) (+ ActionValue (stale Input|EnhancedActionEvents|EnhancedInputActionIA_Turn ActionValue)) -1.0)))
    (bind _output_get_2 (Variables|Default|SetRightWheelForce (Math|Float|Clamp(Float) (- ActionValue (stale Input|EnhancedActionEvents|EnhancedInputActionIA_Turn ActionValue)) -1.0)))
    (Class|PrimitiveComponent|AddForceatLocationLocal (Variables|Default|GetPlayerMesh) (Math|Vector|MakeVector (* _output_get (Variables|Default|GetForceMultiplier)) 0.0 0.0) (Variables|/Script/Engine.SceneComponent|GetRelativeLocation (Variables|Default|GetLeftWheel)) "None")
    (Class|PrimitiveComponent|AddForceatLocationLocal (Variables|Default|GetPlayerMesh) (Math|Vector|MakeVector (* _output_get_2 (Variables|Default|GetForceMultiplier)) 0.0 0.0) (Variables|/Script/Engine.SceneComponent|GetRelativeLocation (Variables|Default|GetRightWheel)) "None"))
  (:Completed
    (Variables|Default|SetLeftWheelForce 0.0)
    (Variables|Default|SetRightWheelForce 0.0)))

(event Input|EnhancedActionEvents|EnhancedInputActionIA_Turn
  (params (ActionValue :type Float%20%28double-precision%29) (ElapsedSeconds :type Float%20%28double-precision%29) (TriggeredSeconds :type Float%20%28double-precision%29) (InputAction :type Input%20Action%20Object%20Reference :default "/Game/MyStuff/Input/IA_Turn.IA_Turn"))
  (:Triggered
    (bind _output_get (Variables|Default|SetLeftWheelForce (Math|Float|Clamp(Float) (+ (stale Input|EnhancedActionEvents|EnhancedInputActionIA_ForwardsBackwards ActionValue) ActionValue) -1.0)))
    (bind _output_get_2 (Variables|Default|SetRightWheelForce (Math|Float|Clamp(Float) (- (stale Input|EnhancedActionEvents|EnhancedInputActionIA_ForwardsBackwards ActionValue) ActionValue) -1.0)))
    (Class|PrimitiveComponent|AddForceatLocationLocal (Variables|Default|GetPlayerMesh) (Math|Vector|MakeVector (* _output_get (Variables|Default|GetForceMultiplier)) 0.0 0.0) (Variables|/Script/Engine.SceneComponent|GetRelativeLocation (Variables|Default|GetLeftWheel)) "None")
    (Class|PrimitiveComponent|AddForceatLocationLocal (Variables|Default|GetPlayerMesh) (Math|Vector|MakeVector (* _output_get_2 (Variables|Default|GetForceMultiplier)) 0.0 0.0) (Variables|/Script/Engine.SceneComponent|GetRelativeLocation (Variables|Default|GetRightWheel)) "None"))
  (:Completed
    (Variables|Default|SetLeftWheelForce 0.0)
    (Variables|Default|SetRightWheelForce 0.0)))

(event EventBeginPlay
  ;[0.15 0.15 0.15 0.5] To Setup IMC to player ( Step 1)
  (Input|AddMappingContext (PlayerController|LocalPlayerSubsystems|GetEnhancedInputLocalPlayerSubsystem (Game|GetPlayerController 0)) "/Game/MyStuff/Input/IMC_Default.IMC_Default" 0 "(bIgnoreAllPressedKeysUntilRelease=True,bForceImmediately=False,bNotifyUserSettings=False)"))

(event Collision|EventActorBeginOverlap
  (params (OtherActor :type Actor%20Object%20Reference)))

(event EventTick
  (params (DeltaSeconds :type Float%20%28single-precision%29)))

(fn ConstructionScript)